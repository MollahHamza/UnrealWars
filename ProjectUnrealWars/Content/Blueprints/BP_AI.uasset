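; BP_AI is an enemy AI pawn that wanders, chases the player's third-person character on sight and shoots with a rifle.
; Wandering repeats random reachable-point moves, while PawnSensing starts a chase that fires once upon arrival.
; Fire spawns a muzzle flash and applies line-trace damage, with the trace end multiplying socket location by scaled up vector rather than adding.
; Damage reduces Health, triggering ragdoll and disabling movement while Health remains above zero.
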(event `self.ReceiveBeginPlay`
  (`self.SearchAround`))

(event `SearchAround`
  (`|AIMoveTo` self (`NavigationSystemV1.K2_GetRandomReachablePointInRadius` (`self.K2_GetActorLocation`) 2000.0 null null) null 300.0
    (:`OnSuccess`
      (`KismetSystemLibrary.Delay` 0.1)
      (`self.SearchAround`))))

(event `self.ReceiveAnyDamage`
  (params (Damage :type "Float (single-precision)") (DamageType :type "DamageType Object Reference") (InstigatedBy :type "Controller Object Reference") (DamageCauser :type "Actor Object Reference"))
  (set `self.Health` (- (`self.Health`) Damage))
  (if (not (<= (`self.Health`) 0.0))
    (`KismetSystemLibrary.PrintString` "Hello")
    (`PrimitiveComponent.SetSimulatePhysics` (`self.Mesh`) true)
    (`CharacterMovementComponent.SetMovementMode` (`self.CharacterMovement`) "MOVE_None" 0)))

(event `self.PawnSensing.OnSeePawn`
  (params (Pawn :type "Pawn Object Reference"))
  (cast `/Game/ThirdPerson/Blueprints/BP_ThirdPersonCharacter` Pawn)
  (`self.chase` Pawn))

(event `chase`
  (params (TargetActor :type "Actor Object Reference"))
  (`|AIMoveTo` self (0.0 0.0 0.0) TargetActor 300.0
    (:`OnSuccess`
      (`KismetSystemLibrary.PrintString` "Hello")
      (`self.Fire` null))))

(event `Fire`
  (params (`Target actor` :type "Actor Object Reference"))
  (bind (_returnvalue_location _returnvalue_rotation) (`KismetMathLibrary.BreakTransform` (`SceneComponent.GetSocketTransform` (`self.Rifle`) "b_gun_muzzleflash" "RTS_World")))
  (`GameplayStatics.SpawnEmitterAttached` "/Game/InfinityBladeEffects/Effects/FX_Monsters/FX_Monster_Gruntling/Master/P_BackPack_MuzzleFlash.P_BackPack_MuzzleFlash" (`self.Rifle`) "b_gun_muzzleflash" _returnvalue_location _returnvalue_rotation (0.1 0.2 0.1) "KeepWorldPosition")
  (bind (_outhit _returnvalue) (`KismetSystemLibrary.LineTraceSingle` :`Start` _returnvalue_location :`End` (* _returnvalue_location (* (`KismetMathLibrary.GetUpVector` _returnvalue_rotation) 3000.0)) :`TraceChannel` "TraceTypeQuery1" :`DrawDebugType` "ForDuration"))
  (if _returnvalue
    (`GameplayStatics.ApplyDamage` (`.HitActor` (`GameplayStatics.BreakHitResult` _outhit)) 1.0)))

(fn `UserConstructionScript`)